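; BP_Gun is a weapon actor that is owned by a shooter character and carries static mesh attachments on its skeletal mesh.
; The construction script gathers all descendant components of exactly the StaticMeshComponent class, disables their collision and stores them in Attachments.
; BeginPlay casts the owner to BP_ShooterCharacter and caches it as OwnerReference.
; No firing or per-frame logic is implemented here.
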(event `self.ReceiveBeginPlay`
  (bind _asbp_shooter_character (cast `/Game/BP_ShooterCharacter` (`self.GetOwner`)))
  (set `self.OwnerReference` _asbp_shooter_character))

(event `self.ReceiveTick`
  (params (DeltaSeconds :type "Float (single-precision)")))

(fn `UserConstructionScript`
  (for _array_element (`SceneComponent.GetChildrenComponents` (`self.SkeletalMesh`) true)
    (bind _asstatic_mesh_component (cast `StaticMeshComponent` _array_element))
    (if (== (`GameplayStatics.GetObjectClass` _array_element) "/Script/Engine.StaticMeshComponent")
      (`PrimitiveComponent.SetCollisionEnabled` _asstatic_mesh_component "NoCollision")
      (`KismetArrayLibrary.Array_Add` (`self.Attachments`) _asstatic_mesh_component))))