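; BP_Bullet is a weapon projectile that reacts to its first hit, then destroys itself.
; On BeginPlay its collision ignores the shooter, found as the owner of the gun that owns the bullet.
; A DoOnce-gated component hit passes the impact to ProjectileOnHit, defined outside this graph, and reports a noise event at that location.
; It then stops movement and destroys the actor after a brief delay.
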(event `self.ReceiveBeginPlay`
  (`PrimitiveComponent.IgnoreActorWhenMoving` (`self.CollisionComponent`) (`self.GetOwner` (`self.GetOwner`)) true))

(event `self.CollisionComponent.OnComponentHit`
  (params (HitComponent :type "PrimitiveComponent Object Reference") (OtherActor :type "Actor Object Reference") (OtherComp :type "PrimitiveComponent Object Reference") (NormalImpulse :type "Vector Structure") (Hit :type "HitResult Structure (by ref)"))
  (`/Engine/EditorBlueprintResources/StandardMacros.DoOnce` false
    (:`Completed`
      (`self.ProjectileOnHit` HitComponent OtherActor OtherComp NormalImpulse Hit)
      (`AISense_Hearing.ReportNoiseEvent` (`.Location` (`GameplayStatics.BreakHitResult` Hit)) 2.0 self 1500.0)
      (`MovementComponent.StopMovementImmediately` (`self.ProjectileMovementComponent`))
      (`KismetSystemLibrary.Delay` 0.05)
      (`self.K2_DestroyActor`))))

(fn `UserConstructionScript`)