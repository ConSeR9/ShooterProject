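; Enemy AI controller that runs the BT_EnemyAI behavior tree and feeds it perception results through the blackboard.
; On begin play it starts the tree, then reacts to AI Perception target updates by sense type.
; Sight sets TargetActor to the seen actor and clears it when sight is lost.
; Any other sense, treated as hearing, writes the stimulus location to TargetLocation.
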(event `self.ReceiveBeginPlay`
  (`self.RunBehaviorTree` "/Game/AI/BT_EnemyAI.BT_EnemyAI"))

(event `self.AIPerception.OnTargetPerceptionUpdated`
  (params (Actor :type "Actor Object Reference") (Stimulus :type "AIStimulus Structure"))
  (bind (_age _expirationage _strength _stimuluslocation _receiverlocation _tag _bsuccessfullysensed) (break `AIStimulus` Stimulus))
  (bind _returnvalue (`AIPerceptionSystem.GetSenseClassForStimulus` Stimulus))
  (if (== _returnvalue "/Script/AIModule.AISense_Sight")
    (if _bsuccessfullysensed
      (`BlackboardComponent.SetValueAsObject` (`self.Blackboard`) "TargetActor" Actor)
      (else
        (`BlackboardComponent.ClearValue` (`self.Blackboard`) "TargetActor")))
    (else
      (`BlackboardComponent.SetValueAsVector` (`self.Blackboard`) "TargetLocation" _stimuluslocation))))

(fn `UserConstructionScript`)